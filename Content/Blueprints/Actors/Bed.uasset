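; Bed actor that highlights under the cursor and switches to a level camera with a bed widget when the player character enters its collision box.
; Cursor hover swaps the mesh material.
; Overlap start casts to Victor_Char and Victor_PC, stops movement, blends the view to CameraToFind and shows the character's BedREF widget; overlap end reverses the view and widget.
; The Interact function only returns false.
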(event `self.Bed.OnBeginCursorOver`
  (params (TouchedComponent :type "PrimitiveComponent Object Reference"))
  ;[1 1 1] Hilight Objects
  (`PrimitiveComponent.SetMaterial` (`self.Bed`) 0 "/Game/Import/Objects_Interior_Village__Demo/Textures/bed_Mat_Inst.bed_Mat_Inst"))

(event `self.Bed.OnEndCursorOver`
  (params (TouchedComponent :type "PrimitiveComponent Object Reference"))
  ;[1 1 1] Hilight Objects
  (`PrimitiveComponent.SetMaterial` (`self.Bed`) 0 "/Game/Import/Objects_Interior_Village__Demo/Textures/bed_Mat.bed_Mat"))

(event `self.CollisionBox.OnComponentBeginOverlap`
  (params (OverlappedComponent :type "PrimitiveComponent Object Reference") (OtherActor :type "Actor Object Reference") (OtherComp :type "PrimitiveComponent Object Reference") (OtherBodyIndex :type Integer) (bFromSweep :type Boolean) (SweepResult :type "HitResult Structure (by ref)"))
  ;[1 1 1] Anchor Char to Location after interaction / Change Main Camera to Level Camera
  (set `self.Other Actor` OtherActor)
  (`self.Cast To Main Charater`)
  (`MovementComponent.StopMovementImmediately` (`Character.CharacterMovement` (`self.CharREF`)))
  (`PlayerController.SetViewTargetWithBlend` (`self.As PC Victor`) (`self.CameraToFind`) 0.2 "VTBlend_Linear" 0.0 false)
  (`UserWidget.AddToViewport` (`/Game/Blueprints/Characters/Victor_Char.BedREF` (`self.CharREF`)) 0))

(event `self.CollisionBox.OnComponentEndOverlap`
  (params (OverlappedComponent :type "PrimitiveComponent Object Reference") (OtherActor :type "Actor Object Reference") (OtherComp :type "PrimitiveComponent Object Reference") (OtherBodyIndex :type Integer))
  ;[1 1 1] Change back to Main Characters Camera
  (`self.Cast To Main Charater`)
  (`PlayerController.SetViewTargetWithBlend` (`self.As PC Victor`) (`self.CharREF`) 0.2 "VTBlend_Linear" 0.0 false)
  (`Widget.RemoveFromParent` (`/Game/Blueprints/Characters/Victor_Char.BedREF` (`self.CharREF`))))

(event `Cast To Main Charater`
  ;[1 1 1] Casting to Main Character & Saving Actors into Variables
  (bind _asplayer_character_victor (cast `/Game/Blueprints/Characters/Victor_Char` (`self.Other Actor`)))
  (set `self.CharREF` _asplayer_character_victor)
  (bind _aspc_victor (cast `/Game/Blueprints/Controller/Victor_PC` (`Pawn.GetController` _asplayer_character_victor)))
  (set `self.As PC Victor` _aspc_victor))

(fn `Interact`
  (params (Interactor :type "PrimitiveComponent Object Reference"))
  (returns (`Interacted?` :type Boolean))
  (return false))

(fn `UserConstructionScript`)