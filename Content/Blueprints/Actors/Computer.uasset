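; Interactive computer desk actor that highlights on cursor hover and switches to a screen view when the player enters its collision box.
; Collapsed cursor graphs funnel every part's hover into shared material swaps for the whole desk set, excluding the chair.
; Overlap caches character and controller, disables chair collision, blends to the computer camera and shows the screen.
; End overlap, marked obsolete, restores collision and view; click outputs have no handlers.
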(event `self.Chair.OnBeginCursorOver`
  (params (TouchedComponent :type "PrimitiveComponent Object Reference"))
  ;[1 1 1] Highlight
  (`PrimitiveComponent.SetMaterial` (`self.All_Table_14`) 0 "/Game/Import/PaqueteDeModelos3/Armchair/Textures/Wood_10_Mat_Inst.Wood_10_Mat_Inst" :!label _label)
  (`PrimitiveComponent.SetMaterial` (`self.SM_ComputerKeyboard_A02_N1`) 0 "/Game/Import/Deko_MatrixDemo/Apartment/Materials/MI_ComputerKeyboard_A02_Inst.MI_ComputerKeyboard_A02_Inst")
  (`PrimitiveComponent.SetMaterial` (`self.SM_ComputerMouse_A01_N1`) 0 "/Game/Import/Deko_MatrixDemo/Apartment/Materials/MI_ComputerMouse_A01_Inst.MI_ComputerMouse_A01_Inst")
  (`PrimitiveComponent.SetMaterial` (`self.SM_BooksPamphlets_E01_N1`) 0 "/Game/Import/Deko_MatrixDemo/Apartment/Materials/MI_Newspaper_WobblyMag_OpenMagTight_A01_Inst.MI_Newspaper_WobblyMag_OpenMagTight_A01_Inst")
  (`PrimitiveComponent.SetMaterial` (`self.SM_ComputerTower_A01_N1`) 0 "/Game/Import/Deko_MatrixDemo/Apartment/Materials/MI_ComputerTower_A01_Inst.MI_ComputerTower_A01_Inst")
  (`PrimitiveComponent.SetMaterial` (`self.SM_ComputerMonitor_A01_N1`) 0 "/Game/Import/Deko_MatrixDemo/Apartment/Materials/MI_ComputerMonitor_A01_Inst.MI_ComputerMonitor_A01_Inst"))

(event `self.SM_ComputerMonitor_A01_N1.OnBeginCursorOver`
  (params (TouchedComponent :type "PrimitiveComponent Object Reference"))
  ;[1 1 1] Highlight
  (goto _label))

(event `self.SM_ComputerTower_A01_N1.OnBeginCursorOver`
  (params (TouchedComponent :type "PrimitiveComponent Object Reference"))
  ;[1 1 1] Highlight
  (goto _label))

(event `self.SM_BooksPamphlets_E01_N1.OnBeginCursorOver`
  (params (TouchedComponent :type "PrimitiveComponent Object Reference"))
  ;[1 1 1] Highlight
  (goto _label))

(event `self.SM_ComputerMouse_A01_N1.OnBeginCursorOver`
  (params (TouchedComponent :type "PrimitiveComponent Object Reference"))
  ;[1 1 1] Highlight
  (goto _label))

(event `self.SM_ComputerKeyboard_A02_N1.OnBeginCursorOver`
  (params (TouchedComponent :type "PrimitiveComponent Object Reference"))
  ;[1 1 1] Highlight
  (goto _label))

(event `self.All_Table_14.OnBeginCursorOver`
  (params (TouchedComponent :type "PrimitiveComponent Object Reference"))
  ;[1 1 1] Highlight
  (goto _label))

(event `self.Chair.OnEndCursorOver`
  (params (TouchedComponent :type "PrimitiveComponent Object Reference"))
  ;[1 1 1] Highlight
  (`PrimitiveComponent.SetMaterial` (`self.All_Table_14`) 0 "/Game/Import/PaqueteDeModelos3/Armchair/Textures/Wood_10_Mat.Wood_10_Mat" :!label _label_2)
  (`PrimitiveComponent.SetMaterial` (`self.SM_ComputerKeyboard_A02_N1`) 0 "/Game/Import/Deko_MatrixDemo/Apartment/Materials/MI_ComputerKeyboard_A02.MI_ComputerKeyboard_A02")
  (`PrimitiveComponent.SetMaterial` (`self.SM_ComputerMouse_A01_N1`) 0 "/Game/Import/Deko_MatrixDemo/Apartment/Materials/MI_ComputerMouse_A01.MI_ComputerMouse_A01")
  (`PrimitiveComponent.SetMaterial` (`self.SM_BooksPamphlets_E01_N1`) 0 "/Game/Import/Deko_MatrixDemo/Apartment/Materials/MI_Newspaper_WobblyMag_OpenMagTight_A01.MI_Newspaper_WobblyMag_OpenMagTight_A01")
  (`PrimitiveComponent.SetMaterial` (`self.SM_ComputerTower_A01_N1`) 0 "/Game/Import/Deko_MatrixDemo/Apartment/Materials/MI_ComputerTower_A01.MI_ComputerTower_A01")
  (`PrimitiveComponent.SetMaterial` (`self.SM_ComputerMonitor_A01_N1`) 0 "/Game/Import/Deko_MatrixDemo/Apartment/Materials/MI_ComputerMonitor_A01.MI_ComputerMonitor_A01"))

(event `self.SM_ComputerMonitor_A01_N1.OnEndCursorOver`
  (params (TouchedComponent :type "PrimitiveComponent Object Reference"))
  ;[1 1 1] Highlight
  (goto _label_2))

(event `self.SM_ComputerTower_A01_N1.OnEndCursorOver`
  (params (TouchedComponent :type "PrimitiveComponent Object Reference"))
  ;[1 1 1] Highlight
  (goto _label_2))

(event `self.SM_BooksPamphlets_E01_N1.OnEndCursorOver`
  (params (TouchedComponent :type "PrimitiveComponent Object Reference"))
  ;[1 1 1] Highlight
  (goto _label_2))

(event `self.SM_ComputerMouse_A01_N1.OnEndCursorOver`
  (params (TouchedComponent :type "PrimitiveComponent Object Reference"))
  ;[1 1 1] Highlight
  (goto _label_2))

(event `self.SM_ComputerKeyboard_A02_N1.OnEndCursorOver`
  (params (TouchedComponent :type "PrimitiveComponent Object Reference"))
  ;[1 1 1] Highlight
  (goto _label_2))

(event `self.All_Table_14.OnEndCursorOver`
  (params (TouchedComponent :type "PrimitiveComponent Object Reference"))
  ;[1 1 1] Highlight
  (goto _label_2))

(event `self.CollisionBox.OnComponentBeginOverlap`
  (params (OverlappedComponent :type "PrimitiveComponent Object Reference") (OtherActor :type "Actor Object Reference") (OtherComp :type "PrimitiveComponent Object Reference") (OtherBodyIndex :type Integer) (bFromSweep :type Boolean) (SweepResult :type "HitResult Structure (by ref)"))
  (set `self.Other Actor` OtherActor)
  ;[1 1 1] Triiger Interact Screen
  (`PrimitiveComponent.SetCollisionEnabled` (`self.Chair`) "NoCollision")
  (`self.Cast To Main Charater`)
  (`PlayerController.SetViewTargetWithBlend` (`self.As PC Victor`) (`self.CameraToFind`) 0.2 "VTBlend_Linear" 0.0 false)
  (`SceneComponent.SetVisibility` (`self.Screen`) true false))

(event `self.Chair.OnClicked`
  (params (TouchedComponent :type "PrimitiveComponent Object Reference") (ButtonPressed :type "Key Structure"))
  ;[1 1 1] Obsolete for now
)

(event `self.SM_ComputerTower_A01_N1.OnClicked`
  (params (TouchedComponent :type "PrimitiveComponent Object Reference") (ButtonPressed :type "Key Structure"))
  ;[1 1 1] Obsolete for now
)

(event `self.SM_ComputerMonitor_A01_N1.OnClicked`
  (params (TouchedComponent :type "PrimitiveComponent Object Reference") (ButtonPressed :type "Key Structure"))
  ;[1 1 1] Obsolete for now
)

(event `self.SM_BooksPamphlets_E01_N1.OnClicked`
  (params (TouchedComponent :type "PrimitiveComponent Object Reference") (ButtonPressed :type "Key Structure"))
  ;[1 1 1] Obsolete for now
)

(event `self.SM_ComputerKeyboard_A02_N1.OnClicked`
  (params (TouchedComponent :type "PrimitiveComponent Object Reference") (ButtonPressed :type "Key Structure"))
  ;[1 1 1] Obsolete for now
)

(event `self.SM_ComputerMouse_A01_N1.OnClicked`
  (params (TouchedComponent :type "PrimitiveComponent Object Reference") (ButtonPressed :type "Key Structure"))
  ;[1 1 1] Obsolete for now
)

(event `self.All_Table_14.OnClicked`
  (params (TouchedComponent :type "PrimitiveComponent Object Reference") (ButtonPressed :type "Key Structure"))
  ;[1 1 1] Obsolete for now
)

(event `self.CollisionBox.OnComponentEndOverlap`
  (params (OverlappedComponent :type "PrimitiveComponent Object Reference") (OtherActor :type "Actor Object Reference") (OtherComp :type "PrimitiveComponent Object Reference") (OtherBodyIndex :type Integer))
  ;[1 1 1] Exit Interaction Screen
  (`PrimitiveComponent.SetCollisionEnabled` (`self.Chair`) "QueryAndPhysics")
  (`self.Cast To Main Charater`)
  (`PlayerController.SetViewTargetWithBlend` (`self.As PC Victor`) (`self.CharREF`) 0.2 "VTBlend_Linear" 0.0 false))

(event `Cast To Main Charater`
  ;[1 1 1] Casting to Main Character & Saving Actors into Variables
  (bind _asplayer_character_victor (cast `/Game/Blueprints/Characters/Victor_Char` (`self.Other Actor`)))
  (set `self.CharREF` _asplayer_character_victor)
  (bind _aspc_victor (cast `/Game/Blueprints/Controller/Victor_PC` (`Pawn.GetController` _asplayer_character_victor)))
  (set `self.As PC Victor` _aspc_victor))

(fn `UserConstructionScript`)