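; Door actor that swings open and closed on interaction or overlap, switching the player's camera as they pass through its trigger.
; Interact sets the timeline play rate from open or close time and toggles direction; the timeline lerps the pivot's yaw and flips Open when finished.
; Overlapping the collision box stops the character, blends to a level-assigned camera and opens the door; leaving blends back to the character and closes it.
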(event `Open Door`
  (bind (_direction _doortrack) (`Timeline|OpenDoorT` :!via `PlayFromStart` :!label _label)
    (:`Update`
      (`SceneComponent.K2_SetRelativeRotation` (`self.DoorPivot`) (`KismetMathLibrary.MakeRotator` 0.0 0.0 (`KismetMathLibrary.Lerp` (`self.ClosePosition`) (`self.OpenPosition`) _doortrack)) false false))
    (:`Finished`
      (set `self.Open?` (not (`self.Open?`))))))

(event `Close Door`
  (goto _label :!via `Reverse`))

(event `self.CollisionBox.OnComponentBeginOverlap`
  (params (OverlappedComponent :type "PrimitiveComponent Object Reference") (OtherActor :type "Actor Object Reference") (OtherComp :type "PrimitiveComponent Object Reference") (OtherBodyIndex :type Integer) (bFromSweep :type Boolean) (SweepResult :type "HitResult Structure (by ref)"))
  ;[1 1 1] Anchor Char to Location after interaction / Change Main Camera to Level Camera
  (set `self.Other Actor` OtherActor)
  (`self.Cast To Main Charater`)
  (`MovementComponent.StopMovementImmediately` (`Character.CharacterMovement` (`self.CharREF`)))
  (`PlayerController.SetViewTargetWithBlend` (`self.Victor_PCREF`) (`self.Camera To Find`) 0.2 "VTBlend_Linear" 0.0 false) ; Camera To Find must be selected at the Actor placed on the level
  (`self.Open Door`))

(event `self.CollisionBox.OnComponentEndOverlap`
  (params (OverlappedComponent :type "PrimitiveComponent Object Reference") (OtherActor :type "Actor Object Reference") (OtherComp :type "PrimitiveComponent Object Reference") (OtherBodyIndex :type Integer))
  ;[1 1 1] Change back to Main Characters Camera
  (`self.Cast To Main Charater`)
  (`PlayerController.SetViewTargetWithBlend` (`self.Victor_PCREF`) (`self.CharREF`) 0.2 "VTBlend_Linear" 0.0 false)
  (`self.Close Door`))

(event `Cast To Main Charater`
  ;[1 1 1] Casting to Main Character & Saving Actors into Variables
  (bind _asplayer_character_victor (cast `/Game/Blueprints/Characters/Victor_Char` (`self.Other Actor`)))
  (set `self.CharREF` _asplayer_character_victor)
  (bind _aspc_victor (cast `/Game/Blueprints/Controller/Victor_PC` (`Pawn.GetController` _asplayer_character_victor)))
  (set `self.Victor_PCREF` _aspc_victor))

(fn `Interact`
  (params (Interactor :type "PrimitiveComponent Object Reference"))
  (returns (`Interacted?` :type Boolean))
  (bind _opendoort (`self.OpenDoorT`))
  (if (not (`self.Open?`))
    (`TimelineComponent.SetPlayRate` _opendoort (/ (`self.TimeToOpen(S)`) 1.0))
    (`self.Open Door`)
    (else
      (`TimelineComponent.SetPlayRate` _opendoort (/ (`self.TimeToClose(S)`) 1.0))
      (`self.Close Door`)))
  (return false))

(fn `UserConstructionScript`)