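; Clickable food actor that the player collects from a completed computer order to stock the refrigerator with meals.
; On BeginPlay it caches the Victor_Char player and the Computer actor's screen widget.
; Clicking the model compares that widget's delivery status and meal name as display text, increments the matching small, medium or large count on the player's fridge reference, then destroys the actor.
; Cursor hover swaps the model's material as a highlight.
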(event `self.ReceiveBeginPlay`
  ;[1 1 1] Initial Setup
  (bind _asvictor_char (cast `/Game/Blueprints/Characters/Victor_Char` (`GameplayStatics.GetPlayerCharacter` 0)))
  (set `self.CharREF` _asvictor_char)
  (bind _returnvalue (`GameplayStatics.GetActorOfClass` "/Game/Blueprints/Actors/Computer.Computer_C"))
  (bind _asmain_computer_screen_ui (cast `/Game/Blueprints/UI/MainComputerScreen_UI` (`WidgetComponent.GetWidget` (`/Game/Blueprints/Actors/Computer.Screen` _returnvalue))))
  (set `self.ComputerUIREF` _asmain_computer_screen_ui))

(event `self.model.OnClicked`
  (params (TouchedComponent :type "PrimitiveComponent Object Reference") (ButtonPressed :type "Key Structure"))
  (bind _result (`|FormatText` "Delivery complete!"))
  (bind _computeruiref (`self.ComputerUIREF`))
  (bind _refriref (`/Game/Blueprints/Characters/Victor_Char.RefriREF` (`self.CharREF`)))
  (bind _refriref_2 (`/Game/Blueprints/Characters/Victor_Char.RefriREF` (`self.CharREF`)))
  (bind _deliverystatus (`/Game/Blueprints/UI/MainComputerScreen_UI.DeliveryStatus` _computeruiref))
  (bind _placeholdertextmeal (`/Game/Blueprints/UI/MainComputerScreen_UI.PlaceholderTextMeal` _computeruiref))
  (bind _refriref_3 (`/Game/Blueprints/Characters/Victor_Char.RefriREF` (`self.CharREF`)))
  ;[1 1 1] Destroy Actor & Add to Meal Amount
  (if (and (== _deliverystatus _result) (== _placeholdertextmeal (`|FormatText` "Small Meal")))
    (set `/Game/Blueprints/UI/Refrigerator_UI.SMealsAmount` (+ (`/Game/Blueprints/UI/Refrigerator_UI.SMealsAmount` _refriref) 1) _refriref)
    (`self.K2_DestroyActor` :!label _label)
    (elif (and (== _deliverystatus _result) (== _placeholdertextmeal (`|FormatText` "Medium Meal")))
      (set `/Game/Blueprints/UI/Refrigerator_UI.MMealsAmount` (+ (`/Game/Blueprints/UI/Refrigerator_UI.MMealsAmount` _refriref_2) 1) _refriref_2)
      (goto _label)
      (elif (and (== _deliverystatus _result) (== _placeholdertextmeal (`|FormatText` "Large Meal")))
        (set `/Game/Blueprints/UI/Refrigerator_UI.LMealsAmount` (+ (`/Game/Blueprints/UI/Refrigerator_UI.LMealsAmount` _refriref_3) 1) _refriref_3)
        (goto _label)))))

(event `self.model.OnBeginCursorOver`
  (params (TouchedComponent :type "PrimitiveComponent Object Reference"))
  ;[1 1 1] Hover
  (`PrimitiveComponent.SetMaterial` (`self.model`) 0 "/Game/Import/Material_001_Inst.Material_001_Inst"))

(event `self.model.OnEndCursorOver`
  (params (TouchedComponent :type "PrimitiveComponent Object Reference"))
  ;[1 1 1] Hover
  (`PrimitiveComponent.SetMaterial` (`self.model`) 0 "/Game/Import/Material_001.Material_001"))

(fn `UserConstructionScript`)