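; Interactive kitchen refrigerator actor, grouped with a microwave and table, that gives the player a close-up view and UI on approach.
; Cursor hover on any part swaps refrigerator and microwave materials to instanced variants, restoring them on exit.
; Collision overlap stops the character, blends to another camera, shows the fridge widget and swings the bottom door open with a timeline.
; Leaving restores the character camera, removes the widget and reverses the door.
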(event `self.Electronics_kitchen_Refrigerator_door.OnBeginCursorOver`
  (params (TouchedComponent :type "PrimitiveComponent Object Reference"))
  (`PrimitiveComponent.SetMaterial` (`self.All_Refrigerator_door_01`) 0 "/Game/Import/PaqueteDeModelos3/Bath_Hygiene/Models/Plastic_06_Inst.Plastic_06_Inst" :!label _label)
  (`PrimitiveComponent.SetMaterial` (`self.Electronics_kitchen_Refrigerator_door`) 0 "/Game/Import/PaqueteDeModelos3/Bath_Hygiene/Models/Plastic_06_Inst.Plastic_06_Inst")
  (`PrimitiveComponent.SetMaterial` (`self.Electronics_kitchen_Refrigerator`) 0 "/Game/Import/PaqueteDeModelos3/Bath_Hygiene/Models/Plastic_06_Inst.Plastic_06_Inst")
  (`PrimitiveComponent.SetMaterial` (`self.All_Refrigerator_door_01`) 1 "/Game/Import/PaqueteDeModelos3/Deds_others/Textures/Metal_04_Mat_Inst.Metal_04_Mat_Inst")
  (`PrimitiveComponent.SetMaterial` (`self.Electronics_kitchen_Refrigerator_door`) 1 "/Game/Import/PaqueteDeModelos3/Deds_others/Textures/Metal_04_Mat_Inst.Metal_04_Mat_Inst")
  (`PrimitiveComponent.SetMaterial` (`self.Electronics_kitchen_Refrigerator`) 1 "/Game/Import/PaqueteDeModelos3/Deds_others/Textures/Metal_04_Mat_Inst.Metal_04_Mat_Inst")
  (`PrimitiveComponent.SetMaterial` (`self.All_Refrigerator_door_01`) 2 "/Game/Import/PaqueteDeModelos3/Bath_Hygiene/Models/Plastic_06_Inst.Plastic_06_Inst")
  (`PrimitiveComponent.SetMaterial` (`self.Electronics_kitchen_Refrigerator_door`) 2 "/Game/Import/PaqueteDeModelos3/Bath_Hygiene/Models/Plastic_06_Inst.Plastic_06_Inst")
  (`PrimitiveComponent.SetMaterial` (`self.Electronics_kitchen_Refrigerator`) 2 "/Game/Import/PaqueteDeModelos3/Bath_Hygiene/Models/Plastic_06_Inst.Plastic_06_Inst")
  (`PrimitiveComponent.SetMaterial` (`self.Microwave_Oven_Microwave_Oven-Door`) 0 "/Game/Import/Texture8x8_Mat_Inst.Texture8x8_Mat_Inst")
  (`PrimitiveComponent.SetMaterial` (`self.Microwave_Oven_Microwave_Oven`) 0 "/Game/Import/Texture8x8_Mat_Inst.Texture8x8_Mat_Inst"))

(event `self.Electronics_kitchen_Refrigerator.OnBeginCursorOver`
  (params (TouchedComponent :type "PrimitiveComponent Object Reference"))
  (goto _label))

(event `self.Microwave_Oven_Microwave_Oven-Door.OnBeginCursorOver`
  (params (TouchedComponent :type "PrimitiveComponent Object Reference"))
  (goto _label))

(event `self.Microwave_Oven_Microwave_Oven.OnBeginCursorOver`
  (params (TouchedComponent :type "PrimitiveComponent Object Reference"))
  (goto _label))

(event `self.Deds_others_Table_36.OnBeginCursorOver`
  (params (TouchedComponent :type "PrimitiveComponent Object Reference"))
  (goto _label))

(event `self.All_Refrigerator_door_01.OnBeginCursorOver`
  (params (TouchedComponent :type "PrimitiveComponent Object Reference"))
  (goto _label))

(event `self.Electronics_kitchen_Refrigerator_door.OnEndCursorOver`
  (params (TouchedComponent :type "PrimitiveComponent Object Reference"))
  (`PrimitiveComponent.SetMaterial` (`self.All_Refrigerator_door_01`) 0 "/Game/Import/PaqueteDeModelos3/All/Models/Plastic_06.Plastic_06" :!label _label_2)
  (`PrimitiveComponent.SetMaterial` (`self.Electronics_kitchen_Refrigerator_door`) 0 "/Game/Import/PaqueteDeModelos3/All/Models/Plastic_06.Plastic_06")
  (`PrimitiveComponent.SetMaterial` (`self.Electronics_kitchen_Refrigerator`) 0 "/Game/Import/PaqueteDeModelos3/All/Models/Plastic_06.Plastic_06")
  (`PrimitiveComponent.SetMaterial` (`self.All_Refrigerator_door_01`) 1 "/Game/Import/PaqueteDeModelos3/Deds_others/Textures/Metal_04_Mat.Metal_04_Mat")
  (`PrimitiveComponent.SetMaterial` (`self.Electronics_kitchen_Refrigerator_door`) 1 "/Game/Import/PaqueteDeModelos3/Deds_others/Textures/Metal_04_Mat.Metal_04_Mat")
  (`PrimitiveComponent.SetMaterial` (`self.Electronics_kitchen_Refrigerator`) 1 "/Game/Import/PaqueteDeModelos3/Deds_others/Textures/Metal_04_Mat.Metal_04_Mat")
  (`PrimitiveComponent.SetMaterial` (`self.All_Refrigerator_door_01`) 2 "/Game/Import/PaqueteDeModelos3/All/Models/Plastic_06.Plastic_06")
  (`PrimitiveComponent.SetMaterial` (`self.Electronics_kitchen_Refrigerator_door`) 2 "/Game/Import/PaqueteDeModelos3/All/Models/Plastic_06.Plastic_06")
  (`PrimitiveComponent.SetMaterial` (`self.Electronics_kitchen_Refrigerator`) 2 "/Game/Import/PaqueteDeModelos3/All/Models/Plastic_06.Plastic_06")
  (`PrimitiveComponent.SetMaterial` (`self.Microwave_Oven_Microwave_Oven`) 0 "/Game/Import/Texture8x8_Mat.Texture8x8_Mat")
  (`PrimitiveComponent.SetMaterial` (`self.Microwave_Oven_Microwave_Oven-Door`) 0 "/Game/Import/Texture8x8_Mat.Texture8x8_Mat"))

(event `self.All_Refrigerator_door_01.OnEndCursorOver`
  (params (TouchedComponent :type "PrimitiveComponent Object Reference"))
  (goto _label_2))

(event `self.Deds_others_Table_36.OnEndCursorOver`
  (params (TouchedComponent :type "PrimitiveComponent Object Reference"))
  (goto _label_2))

(event `self.Microwave_Oven_Microwave_Oven.OnEndCursorOver`
  (params (TouchedComponent :type "PrimitiveComponent Object Reference"))
  (goto _label_2))

(event `self.Microwave_Oven_Microwave_Oven-Door.OnEndCursorOver`
  (params (TouchedComponent :type "PrimitiveComponent Object Reference"))
  (goto _label_2))

(event `self.Electronics_kitchen_Refrigerator.OnEndCursorOver`
  (params (TouchedComponent :type "PrimitiveComponent Object Reference"))
  (goto _label_2))

(event `Open Door`
  ;[1 1 1] Open/Close Door Animation
  (bind (_direction _doortrack) (`Timeline|Open/Close Door T` :!via `PlayFromStart` :!label _label_3)
    (:`Update`
      (`SceneComponent.K2_SetRelativeRotation` (`self.DoorPivotBottom`) (`KismetMathLibrary.MakeRotator` 0.0 0.0 (`KismetMathLibrary.Lerp` (`self.ClosePosition`) (`self.OpenPosition`) _doortrack)) false false))
    (:`Finished`
      (set `self.Open?` (not (`self.Open?`))))))

(event `Close Door`
  ;[1 1 1] Open/Close Door Animation
  (goto _label_3 :!via `Reverse`))

(event `self.CollisionBox.OnComponentBeginOverlap`
  (params (OverlappedComponent :type "PrimitiveComponent Object Reference") (OtherActor :type "Actor Object Reference") (OtherComp :type "PrimitiveComponent Object Reference") (OtherBodyIndex :type Integer) (bFromSweep :type Boolean) (SweepResult :type "HitResult Structure (by ref)"))
  ;[1 1 1] Anchor Char to Location after interaction / Change Main Camera to Level Camera
  (set `self.Other Actor` OtherActor)
  (`self.Cast To Main Charater`)
  (`MovementComponent.StopMovementImmediately` (`Character.CharacterMovement` (`self.CharREF`)))
  (`PlayerController.SetViewTargetWithBlend` (`self.Victor_PCREF`) (`self.Camera To Find`) 0.2 "VTBlend_Linear" 0.0 false)
  (`self.Open Door`)
  (`UserWidget.AddToViewport` (`/Game/Blueprints/Characters/Victor_Char.RefriREF` (`self.CharREF`)) 0))

(event `self.CollisionBox.OnComponentEndOverlap`
  (params (OverlappedComponent :type "PrimitiveComponent Object Reference") (OtherActor :type "Actor Object Reference") (OtherComp :type "PrimitiveComponent Object Reference") (OtherBodyIndex :type Integer))
  ;[1 1 1] Change back to Main Characters Camera
  (`self.Cast To Main Charater`)
  (`PlayerController.SetViewTargetWithBlend` (`self.Victor_PCREF`) (`self.CharREF`) 0.2 "VTBlend_Linear" 0.0 false)
  (`self.Close Door`)
  (`Widget.RemoveFromParent` (`/Game/Blueprints/Characters/Victor_Char.RefriREF` (`self.CharREF`))))

(event `self.Microwave_Oven_Microwave_Oven-Door.OnClicked`
  (params (TouchedComponent :type "PrimitiveComponent Object Reference") (ButtonPressed :type "Key Structure"))
  ;[1 1 1] Obsolete for now
)

(event `self.Microwave_Oven_Microwave_Oven.OnClicked`
  (params (TouchedComponent :type "PrimitiveComponent Object Reference") (ButtonPressed :type "Key Structure"))
  ;[1 1 1] Obsolete for now
)

(event `self.Deds_others_Table_36.OnClicked`
  (params (TouchedComponent :type "PrimitiveComponent Object Reference") (ButtonPressed :type "Key Structure"))
  ;[1 1 1] Obsolete for now
)

(event `self.All_Refrigerator_door_01.OnClicked`
  (params (TouchedComponent :type "PrimitiveComponent Object Reference") (ButtonPressed :type "Key Structure"))
  ;[1 1 1] Obsolete for now
)

(event `self.Electronics_kitchen_Refrigerator.OnClicked`
  (params (TouchedComponent :type "PrimitiveComponent Object Reference") (ButtonPressed :type "Key Structure"))
  ;[1 1 1] Obsolete for now
)

(event `self.Electronics_kitchen_Refrigerator_door.OnClicked`
  (params (TouchedComponent :type "PrimitiveComponent Object Reference") (ButtonPressed :type "Key Structure"))
  ;[1 1 1] Obsolete for now
)

(event `Cast To Main Charater`
  ;[1 1 1] Casting to Main Character & Saving Actors into Variables
  (bind _asplayer_character_victor (cast `/Game/Blueprints/Characters/Victor_Char` (`self.Other Actor`)))
  (set `self.CharREF` _asplayer_character_victor)
  (bind _aspc_victor (cast `/Game/Blueprints/Controller/Victor_PC` (`Pawn.GetController` _asplayer_character_victor)))
  (set `self.Victor_PCREF` _aspc_victor))

(fn `UserConstructionScript`)