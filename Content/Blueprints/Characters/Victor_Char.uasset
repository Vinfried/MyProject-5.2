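; Victor_Char is the player character for point-and-click movement, looking around and using in-world screens with the mouse.
; Interact moves Victor to the pawn under the cursor, look keys turn him in timeline-driven quarter steps, and ReturnToCenter walks him back.
; Tick eases the camera toward the cursor within a clamp.
; Overlapping an actor hides the mesh, blocks turning and interacting, and aligns a WidgetInteraction component to the mouse ray for clicks.
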(event `Start Game`
  (`/Engine/EditorBlueprintResources/StandardMacros.FlipFlop`
    (:`A`
      (set `self.StartGame` true))
    (:`B`
      (set `self.StartGame` false))))

(event `self.ReceiveBeginPlay`
  ;[1 1 1] Initial Setup
  (`|ExecutionSequence`
    (:`then_0`
      (if (`self.StartGame`)
        (bind _returnvalue (`|CreateWidget` "/Game/Blueprints/UI/Main_UI.Main_UI_C"))
        (`UserWidget.AddToViewport` _returnvalue 0)
        (bind _returnvalue_2 (`|CreateWidget` "/Game/Blueprints/UI/Refrigerator_UI.Refrigerator_UI_C"))
        (set `self.RefriREF` _returnvalue_2)
        (bind _returnvalue_3 (`|CreateWidget` "/Game/Blueprints/UI/Bed_UI.Bed_UI_C"))
        (set `self.BedREF` _returnvalue_3)
        (bind _returnvalue_4 (`GameplayStatics.GetActorOfClass` "/Game/Blueprints/Actors/Computer.Computer_C"))
        (bind _asmain_computer_screen_ui (cast `/Game/Blueprints/UI/MainComputerScreen_UI` (`WidgetComponent.GetWidget` (`/Game/Blueprints/Actors/Computer.Screen` _returnvalue_4))))
        (set `self.ScreenUIREF` _asmain_computer_screen_ui)))
    (:`then_1`
      (bind _asvictor_pc (cast `/Game/Blueprints/Controller/Victor_PC` (`self.GetController`)))
      (`EnhancedInputSubsystemInterface.AddMappingContext` (pcsubsystem `EnhancedInputLocalPlayerSubsystem` _asvictor_pc) "/Game/Blueprints/Input/IMC_Victor.IMC_Victor" 0 (struct)))))

(event `self.ReceiveTick`
  (params (DeltaSeconds :type "Float (single-precision)"))
  (bind _returnvalue (`GameplayStatics.GetPlayerController` 0))
  (bind _camera (`self.Camera`))
  (bind _widgetinteraction (`self.WidgetInteraction`))
  (bind _camera_2 (`self.Camera`))
  (bind (_returnvalue_roll _returnvalue_pitch _returnvalue_yaw) (`KismetMathLibrary.BreakRotator` (`SceneComponent.K2_GetComponentRotation` (`self.Camera`))))
  (bind (_returnvalue_roll_2 _returnvalue_pitch_2 _returnvalue_yaw_2) (`KismetMathLibrary.BreakRotator` (`SceneComponent.K2_GetComponentRotation` _camera_2)))
  (bind (_returnvalue_roll_3 _returnvalue_pitch_3 _returnvalue_yaw_3) (`KismetMathLibrary.BreakRotator` (`SceneComponent.K2_GetComponentRotation` (`self.CapsuleComponent`))))
  (bind (_returnvalue_roll_4 _returnvalue_pitch_4 _returnvalue_yaw_4) (`KismetMathLibrary.BreakRotator` (`SceneComponent.K2_GetComponentRotation` _camera_2)))
  (bind (_locationx _locationy) (`PlayerController.GetMousePosition` _returnvalue))
  (bind (_worldlocation _worlddirection) (`PlayerController.DeprojectScreenPositionToWorld` _returnvalue _locationx _locationy))
  ;[1 1 1] Start Point for Tick Events
  (`|ExecutionSequence`
    (:`then_0`
      ;[1 1 1] Clamp Camera View
      (if (or (or (< _returnvalue_pitch_2 -10.0) (< _returnvalue_yaw_2 -10.0)) (or (> _returnvalue_pitch_4 10.0) (> _returnvalue_yaw_4 10.0)))
        (`SceneComponent.K2_SetWorldRotation` (`self.Camera`) (`KismetMathLibrary.MakeRotator` 0.0 (`KismetMathLibrary.FClamp` _returnvalue_pitch (- _returnvalue_pitch_3 10.0) (+ _returnvalue_pitch_3 10.0)) (`KismetMathLibrary.FClamp` _returnvalue_yaw (- _returnvalue_yaw_3 10.0) (+ _returnvalue_yaw_3 10.0))) false false)))
    (:`then_1`
      ;[1 1 1] Camera Work
      (bind (_direction _newtrack_0) (`Timeline|LookAround T` :!via `PlayFromStart`)
        (:`Update`
          (`SceneComponent.K2_SetWorldRotation` _camera (`KismetMathLibrary.RLerp` (`SceneComponent.K2_GetComponentRotation` _camera) (`KismetMathLibrary.FindLookAtRotation` (`SceneComponent.K2_GetComponentLocation` _camera) (`PlayerController.DeprojectMousePositionToWorld` (`GameplayStatics.GetPlayerController` 0))) _newtrack_0) false false))))
    (:`then_2`
      ;[1 1 1] Widget Interaction w/ Mouse
      (if (`self.Overlapping`)
        (`SceneComponent.K2_SetWorldLocation` _widgetinteraction _worldlocation false false)
        (`SceneComponent.K2_SetWorldRotation` _widgetinteraction (`KismetMathLibrary.Quat_Rotator` (`KismetMathLibrary.Conv_VectorToQuaternion` _worlddirection)) false false)))
    (:`then_3`
      (if (`self.MovingToLocation`)
        (`GameplayStatics.PlaySoundAtLocation` "/Game/Sounds/Squeaky-Wooden-Floor-Foosteps--Running--www_fesliyanstudios_com.Squeaky-Wooden-Floor-Foosteps--Running--www_fesliyanstudios_com" (`self.K2_GetActorLocation` (`GameplayStatics.GetPlayerCharacter` 0)) (struct) 1.0 1.0 0.0 null null null null)))))

(event `Key|LeftMouseButton`
  (params (Key :type "Key Structure"))
  (bind _widgetinteraction (`self.WidgetInteraction`))
  ;[1 1 1] Widget Interaction w/ Mouse
  (:`Pressed`
    (`WidgetInteractionComponent.PressPointerKey` _widgetinteraction "LeftMouseButton"))
  (:`Released`
    (`WidgetInteractionComponent.ReleasePointerKey` _widgetinteraction "LeftMouseButton")))

(event `EnhancedInput|/Game/Blueprints/Input/IA_Interact`
  (params (ActionValue :type Boolean) (ElapsedSeconds :type "Float (double-precision)") (TriggeredSeconds :type "Float (double-precision)") (InputAction :type "InputAction Object Reference" :default "/Game/Blueprints/Input/IA_Interact.IA_Interact"))
  (bind (_worldlocation _worlddirection) (`PlayerController.DeprojectMousePositionToWorld` (`GameplayStatics.GetPlayerController` 0)))
  ;[1 1 1] Movement Mechanics
  (:`Started`
    (if (not (`self.Overlapping`))
      (`KismetSystemLibrary.LineTraceSingle` :`Start` _worldlocation :`End` (+ _worldlocation (* _worlddirection 5000.0)) :`TraceChannel` "TraceTypeQuery1" :`DrawDebugType` "ForDuration" :`DrawTime` 3.0)
      (if (not (`self.MovingToLocation`))
        (set `self.MovingToLocation` true)
        (`self.Move to Actor` null)
        (set `self.MovingToLocation` false)))))

(event `self.ReceiveActorBeginOverlap`
  (params (OtherActor :type "Actor Object Reference"))
  ;[1 1 1] Set Overlapping Bool
  (set `self.Overlapping` true)
  (`SceneComponent.SetVisibility` (`self.Mesh`) false false))

(event `self.ReceiveActorEndOverlap`
  (params (OtherActor :type "Actor Object Reference"))
  ;[1 1 1] Set Overlapping Bool
  (set `self.Overlapping` false)
  (`SceneComponent.SetVisibility` (`self.Mesh`) true false))

(event `EnhancedInput|/Game/Blueprints/Input/IA_ReturnToCenter`
  (params (ActionValue :type Boolean) (ElapsedSeconds :type "Float (double-precision)") (TriggeredSeconds :type "Float (double-precision)") (InputAction :type "InputAction Object Reference" :default "/Game/Blueprints/Input/IA_ReturnToCenter.IA_ReturnToCenter"))
  ;[1 1 1] Movement Mechanics
  (:`Triggered`
    (`self.Get Actor`)
    (`AIBlueprintHelperLibrary.SimpleMoveToLocation` (`self.GetController`) (`self.Reset Location`))
    ;[1 1 1] Character Rotation
    (bind (_direction _rotation) (`Timeline|Rotate 90 T` :!via `PlayFromStart` :!label _label)
      (:`Update`
        (bind _returnvalue (`KismetMathLibrary.Lerp` (`self.Current Rotation`) (`self.New Rotation`) _rotation))
        (`SceneComponent.K2_SetWorldRotation` (`self.CapsuleComponent`) (`KismetMathLibrary.MakeRotator` 0.0 0.0 _returnvalue) false false)
        (set `self.Current Rotation` _returnvalue)))))

(event `EnhancedInput|/Game/Blueprints/Input/IA_LookRight`
  (params (ActionValue :type Boolean) (ElapsedSeconds :type "Float (double-precision)") (TriggeredSeconds :type "Float (double-precision)") (InputAction :type "InputAction Object Reference" :default "/Game/Blueprints/Input/IA_LookRight.IA_LookRight"))
  (bind (_returnvalue_roll _returnvalue_pitch _returnvalue_yaw) (`KismetMathLibrary.BreakRotator` (`SceneComponent.K2_GetComponentRotation` (`self.Camera`))))
  (bind (_returnvalue_roll_2 _returnvalue_pitch_2 _returnvalue_yaw_2) (`KismetMathLibrary.BreakRotator` (`SceneComponent.K2_GetComponentRotation` (`self.CapsuleComponent`))))
  ;[1 1 1] Character Rotation
  (:`Started`
    (if (not (`self.Rotating`))
      (`|ExecutionSequence`
        (:`then_0`
          (set `self.Rotating` true)
          (`/Engine/EditorBlueprintResources/StandardMacros.DoOnce` false :!label _label_2
            (:`Completed`
              (if (not (`self.Overlapping`))
                (if (!= _returnvalue_yaw _returnvalue_yaw_2)
                  (`SceneComponent.K2_SetWorldRotation` (`self.Camera`) (`KismetMathLibrary.MakeRotator` 0.0 0.0 _returnvalue_yaw_2) false false))
                (`|ExecutionSequence`
                  (:`then_0`
                    (set `self.New Rotation` (+ (`self.Current Rotation`) 90.0)))
                  (:`then_1`
                    (goto _label :!via `PlayFromStart`)))))))
        (:`then_1`
          (`KismetSystemLibrary.Delay` 0.5)
          (set `self.Rotating` false)
          (goto _label_2 :!via `Reset`))))))

(event `EnhancedInput|/Game/Blueprints/Input/IA_LookLeft`
  (params (ActionValue :type Boolean) (ElapsedSeconds :type "Float (double-precision)") (TriggeredSeconds :type "Float (double-precision)") (InputAction :type "InputAction Object Reference" :default "/Game/Blueprints/Input/IA_LookLeft.IA_LookLeft"))
  (bind (_returnvalue_roll _returnvalue_pitch _returnvalue_yaw) (`KismetMathLibrary.BreakRotator` (`SceneComponent.K2_GetComponentRotation` (`self.CapsuleComponent`))))
  (bind (_returnvalue_roll_2 _returnvalue_pitch_2 _returnvalue_yaw_2) (`KismetMathLibrary.BreakRotator` (`SceneComponent.K2_GetComponentRotation` (`self.Camera`))))
  ;[1 1 1] Character Rotation
  (:`Started`
    (if (not (`self.Rotating`))
      (`|ExecutionSequence`
        (:`then_0`
          (set `self.Rotating` true)
          (`/Engine/EditorBlueprintResources/StandardMacros.DoOnce` false :!label _label_3
            (:`Completed`
              (if (not (`self.Overlapping`))
                (if (!= _returnvalue_yaw_2 _returnvalue_yaw)
                  (`SceneComponent.K2_SetWorldRotation` (`self.Camera`) (`KismetMathLibrary.MakeRotator` 0.0 0.0 _returnvalue_yaw) false false))
                (`|ExecutionSequence`
                  (:`then_0`
                    (set `self.New Rotation` (- (`self.Current Rotation`) 90.0)))
                  (:`then_1`
                    (goto _label :!via `PlayFromStart`)))))))
        (:`then_1`
          (`KismetSystemLibrary.Delay` 0.5)
          (set `self.Rotating` false)
          (goto _label_3 :!via `Reset`))))))

(fn `Get Actor`
  (returns (Actor :type "Actor Object Reference"))
  (return (`.HitActor` (`GameplayStatics.BreakHitResult` (`PlayerController.GetHitResultUnderCursorForObjects` (`GameplayStatics.GetPlayerController` 0) (`|MakeArray` "ObjectTypeQuery3" :!type "EObjectTypeQuery Enum") true)))))

(fn `Get Destination`
  (returns (Destination :type "Vector Structure"))
  (return (`.Location` (`GameplayStatics.BreakHitResult` (`PlayerController.GetHitResultUnderCursorByChannel` (`GameplayStatics.GetPlayerController` 0) "TraceTypeQuery1" true)))))

(fn `LookAround`)

(fn `Move to Actor`
  (params (Actor :type "Actor Object Reference"))
  (bind _actor (`self.Get Actor`))
  (`AIBlueprintHelperLibrary.SimpleMoveToActor` (`GameplayStatics.GetPlayerController` 0) _actor))

(fn `Move to Destination`
  (locals (Destination :type "Vector Structure"))
  (bind _charactermovement (`self.CharacterMovement`))
  (bind _destination (`self.Get Destination`))
  (set `local.Destination` _destination)
  (if (> (`KismetMathLibrary.VSize` (- (`self.K2_GetActorLocation`) (`local.Destination`))) 150.0)
    (set `CharacterMovementComponent.MaxWalkSpeed` 600.0 _charactermovement)
    (else
      (set `CharacterMovementComponent.MaxWalkSpeed` 150.0 _charactermovement)))
  (`AIBlueprintHelperLibrary.SimpleMoveToLocation` (`GameplayStatics.GetPlayerController` 0) (`local.Destination`))
  (return))

(fn `UserConstructionScript`)