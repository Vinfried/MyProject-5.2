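; Survival stats component that tracks hunger, fatigue, funds and an in-game clock for the Victor character's levels.
; BeginPlay takes funds and drain rates from LevelVariables_GI; while the game runs, Tick uses Delays to throttle hunger and fatigue drain.
; Any depleted stat shows the lose screen, while reaching hour 20 shows the win screen, flags the level cleared and saves.
; Setter events apply action effects, with time skips also advancing screen-UI training and delivery progress.
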(event `self.ReceiveTick`
  (params (DeltaSeconds :type "Float (single-precision)"))
  (if (`/Game/Blueprints/Characters/Victor_Char.StartGame` (`self.CharREF`))
    (`self.Drain Fatigue`)
    (`self.Drain Hunger`)
    (if (or (<= (`self.Hunger`) 0.0) (<= (`self.Funds`) 0) (<= (`self.Fatigue`) 0.0))
      (`self.Lose`)
      (elif (>= (`self.Hours`) 20)
        (`self.Win`)
        (set `/Game/Blueprints/Characters/Victor_Char.StartGame` false (`self.CharREF`))
        (bind _returnvalue (`GameplayStatics.LoadGameFromSlot` "VictorSlot"))
        (bind _assave_game_victor (cast `` _returnvalue))
        (bind _aslevel_variables_gi (cast `/Game/Blueprints/GameInstances/LevelVariables_GI` (`GameplayStatics.GetGameInstance`)))
        (set `/Game/Blueprints/GameInstances/LevelVariables_GI.Level1Cleared` (`/Game/Blueprints/Components/Stats_Component.Level1Clear` _assave_game_victor) _aslevel_variables_gi)
        (set `/Game/Blueprints/GameInstances/LevelVariables_GI.Level2Cleared` (`/Game/Blueprints/Components/Stats_Component.Level2Clear` _assave_game_victor) _aslevel_variables_gi)
        (set `/Game/Blueprints/GameInstances/LevelVariables_GI.Level3Cleared` (`/Game/Blueprints/Components/Stats_Component.Level3Clear` _assave_game_victor) _aslevel_variables_gi)))))

(event `self.ReceiveBeginPlay`
  ;[1 1 1] Add/Drain Stats
  (bind _aslevel_variables_gi (cast `/Game/Blueprints/GameInstances/LevelVariables_GI` (`GameplayStatics.GetGameInstance`)))
  (set `self.LevelGI` _aslevel_variables_gi)
  (set `self.Funds` (`/Game/Blueprints/GameInstances/LevelVariables_GI.Funds` _aslevel_variables_gi))
  (set `self.HungerDropRate` (`/Game/Blueprints/GameInstances/LevelVariables_GI.HungerDR` _aslevel_variables_gi))
  (set `self.FatigueDropRate` (`/Game/Blueprints/GameInstances/LevelVariables_GI.FatigueDR` _aslevel_variables_gi))
  (set `self.Hunger` (`self.Max Hunger`))
  (set `self.Fatigue` (`self.Max Fatigue`))
  (bind _asvictor_char (cast `/Game/Blueprints/Characters/Victor_Char` (`GameplayStatics.GetPlayerCharacter` 0)))
  (set `self.CharREF` _asvictor_char))

(event `Drain Hunger`
  ;[1 1 1] Add/Drain Stats
  (`KismetSystemLibrary.Delay` 1.0)
  (set `self.Hunger` (`KismetMathLibrary.FClamp` (- (`self.Hunger`) (`self.HungerDropRate`)) 0.0 (`self.Max Hunger`))))

(event `Drain Fatigue`
  ;[1 1 1] Add/Drain Stats
  (`KismetSystemLibrary.Delay` 2.0)
  (set `self.Fatigue` (`KismetMathLibrary.FClamp` (- (`self.Fatigue`) (`self.FatigueDropRate`)) 0.0 (`self.Max Fatigue`))))

(event `TIme`
  (bind _hours (`self.Hours`))
  ;[1 1 1] Timer System
  (`|ExecutionSequence`
    (:`then_0`
      (if (< _hours 20)
        (goto _label :!via `Reset`)))
    (:`then_1`
      (`/Engine/EditorBlueprintResources/StandardMacros.DoOnce` false :!label _label
        (:`Completed`
          (if (>= _hours 20)
            (set `self.Hours` 8)
            (set `self.Minutes` 0)
            (else
              (`KismetSystemLibrary.Delay` 0.25)
              (if (>= (`self.Minutes`) 60)
                (set `self.Minutes` 0)
                (set `self.Hours` (+ (`self.Hours`) 1))
                (else
                  (set `self.Minutes` (+ (`self.Minutes`) 1)))))))))))

(event `Win`
  (bind _savegiref (`self.SaveGIREF`))
  (bind _levelgi (`self.LevelGI`))
  (bind _level (`/Game/Blueprints/GameInstances/LevelVariables_GI.Level` (`self.LevelGI`)))
  ;[1 1 1] Win!
  (bind _returnvalue (`|CreateWidget` "/Game/Blueprints/UI/WinScreen_UI.WinScreen_UI_C"))
  (`UserWidget.AddToViewport` _returnvalue 0)
  (bind _assave_game_gi (cast `/Game/Blueprints/GameInstances/SaveGame_GI` (`GameplayStatics.GetGameInstance`)))
  (set `self.SaveGIREF` _assave_game_gi)
  (if (== _level 0)
    (set `/Game/Blueprints/GameInstances/LevelVariables_GI.Level1Cleared` true _levelgi)
    (`/Game/Blueprints/GameInstances/LevelVariables_GI.Save` _levelgi :!label _label_2)
    (set `/Game/Blueprints/Characters/Victor_Char.StartGame` false (`self.CharREF`))
    (set `self.Hours` 0)
    (set `self.Minutes` 0)
    (`KismetSystemLibrary.PrintText` (`|FormatText` "Level1: {1} \nLevel2: {2} \nLevel3: {3}" (`/Game/Blueprints/GameInstances/SaveGame_GI.Level1Cleared` _savegiref) (`/Game/Blueprints/GameInstances/SaveGame_GI.Level2Cleared` _savegiref) (`/Game/Blueprints/GameInstances/SaveGame_GI.Level3Cleared` _savegiref)))
    (elif (== _level 1)
      (set `/Game/Blueprints/GameInstances/LevelVariables_GI.Level2Cleared` true _levelgi)
      (goto _label_2)
      (elif (== _level 2)
        (set `/Game/Blueprints/GameInstances/LevelVariables_GI.Level3Cleared` true _levelgi)
        (goto _label_2)))))

(event `Lose`
  ;[1 1 1] Lose
  (bind _returnvalue (`|CreateWidget` "/Game/Blueprints/UI/LoseScreen_UI.LoseScreen_UI_C"))
  (`UserWidget.AddToViewport` _returnvalue 0)
  (set `/Game/Blueprints/Characters/Victor_Char.StartGame` false (`self.CharREF`))
  (set `self.Hours` 0)
  (set `self.Minutes` 0))

(event `Set Hunger`
  (params (Value :type "Float (double-precision)"))
  ;[1 1 1] Set Stats based on action
  (set `self.Hunger` (`KismetMathLibrary.FClamp` (+ Value (`self.Hunger`)) 0.0 (`self.Max Hunger`))))

(event `Set Fatigue`
  (params (Value :type "Float (double-precision)"))
  ;[1 1 1] Set Stats based on action
  (set `self.Fatigue` (`KismetMathLibrary.FClamp` (+ Value (`self.Fatigue`)) 0.0 (`self.Max Fatigue`))))

(event `Set Funds`
  (params (Value :type Integer))
  ;[1 1 1] Set Stats based on action
  (set `self.Funds` (+ Value (`self.Funds`))))

(event `Set Hours`
  (params (Value :type Integer) (AITime :type "Float (double-precision)") (DeliveryTime :type "Float (double-precision)"))
  (bind _screenuiref (`/Game/Blueprints/Characters/Victor_Char.ScreenUIREF` (`self.CharREF`)))
  (bind _screenuiref_2 (`/Game/Blueprints/Characters/Victor_Char.ScreenUIREF` (`self.CharREF`)))
  (bind _screenuiref_3 (`/Game/Blueprints/Characters/Victor_Char.ScreenUIREF` (`self.CharREF`)))
  (bind _screenuiref_4 (`/Game/Blueprints/Characters/Victor_Char.ScreenUIREF` (`self.CharREF`)))
  (bind _screenuiref_5 (`/Game/Blueprints/Characters/Victor_Char.ScreenUIREF` (`self.CharREF`)))
  (bind _trainingtime (`/Game/Blueprints/UI/MainComputerScreen_UI.TrainingTime` _screenuiref_4))
  (bind _deliverytime (`/Game/Blueprints/UI/MainComputerScreen_UI.DeliveryTime` _screenuiref))
  ;[1 1 1] Set Stats based on action
  (`|ExecutionSequence`
    (:`then_0`
      (set `self.Hours` (+ Value (`self.Hours`)))
      (if (or (`/Game/Blueprints/UI/MainComputerScreen_UI.TrainingBasic` _screenuiref_5) (`/Game/Blueprints/UI/MainComputerScreen_UI.TrainingFruits` _screenuiref_5) (`/Game/Blueprints/UI/MainComputerScreen_UI.TrainingFacial` _screenuiref_5))
        (set `/Game/Blueprints/UI/MainComputerScreen_UI.TrainingTime` (+ (`KismetMathLibrary.FClamp` AITime 0.0 (`/Game/Blueprints/UI/MainComputerScreen_UI.TimeToComplete` _screenuiref_4)) _trainingtime) _screenuiref_2)
        (if (>= _trainingtime 100.0)
          (set `/Game/Blueprints/UI/MainComputerScreen_UI.TrainingTime` 100.0 _screenuiref_2))))
    (:`then_1`
      (if (`/Game/Blueprints/UI/MainComputerScreen_UI.DeliveryEnRoute` _screenuiref_5)
        (set `/Game/Blueprints/UI/MainComputerScreen_UI.DeliveryTime` (+ (`KismetMathLibrary.FClamp` DeliveryTime 0.0 (`/Game/Blueprints/UI/MainComputerScreen_UI.DeliveryComplete` _screenuiref)) _deliverytime) _screenuiref_3)
        (if (>= _deliverytime 100.0)
          (set `/Game/Blueprints/UI/MainComputerScreen_UI.DeliveryTime` 100.0 _screenuiref_3))))))

(event `Set Minutes`
  (params (Value :type Integer) (Time :type "Float (double-precision)"))
  (bind _screenuiref (`/Game/Blueprints/Characters/Victor_Char.ScreenUIREF` (`self.CharREF`)))
  (bind _screenuiref_2 (`/Game/Blueprints/Characters/Victor_Char.ScreenUIREF` (`self.CharREF`)))
  (bind _screenuiref_3 (`/Game/Blueprints/Characters/Victor_Char.ScreenUIREF` (`self.CharREF`)))
  ;[1 1 1] Set Stats based on action
  (set `self.Minutes` (+ Value (`self.Minutes`)))
  (if (or (`/Game/Blueprints/UI/MainComputerScreen_UI.TrainingBasic` _screenuiref_3) (`/Game/Blueprints/UI/MainComputerScreen_UI.TrainingFruits` _screenuiref_3) (`/Game/Blueprints/UI/MainComputerScreen_UI.TrainingFacial` _screenuiref_3))
    (set `/Game/Blueprints/UI/MainComputerScreen_UI.TrainingTime` (+ (`KismetMathLibrary.FClamp` Time 0.0 (`/Game/Blueprints/UI/MainComputerScreen_UI.TimeToComplete` _screenuiref_2)) (`/Game/Blueprints/UI/MainComputerScreen_UI.TrainingTime` _screenuiref_2)) _screenuiref)
    (if (>= 0.0 100.0)
      (set `/Game/Blueprints/UI/MainComputerScreen_UI.TrainingTime` 100.0 _screenuiref))))