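; Game instance that holds player stats and level-clear progress.
; LevelVariables copies Level, Funds and the hunger and fatigue drop rates from the Stats_Component on the Victor_Char player.
; Save creates a fresh save game object, writes the three level-cleared flags into it and saves it to the VictorSlot slot.
; The copied stats are not written to the save, and no load logic is present.
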(fn `LevelVariables`
  (bind _asvictor_char (cast `/Game/Blueprints/Characters/Victor_Char` (`GameplayStatics.GetPlayerCharacter` 0)))
  (bind _returnvalue (`Actor.GetComponentByClass` _asvictor_char "/Game/Blueprints/Components/Stats_Component.Stats_Component_C"))
  (set `self.Level` (`/Game/Blueprints/Components/Stats_Component.Level` _returnvalue))
  (set `self.Funds` (`/Game/Blueprints/Components/Stats_Component.Funds` _returnvalue))
  (set `self.HungerDR` (`/Game/Blueprints/Components/Stats_Component.HungerDropRate` _returnvalue))
  (set `self.FatigueDR` (`/Game/Blueprints/Components/Stats_Component.FatigueDropRate` _returnvalue)))

(fn `Save`
  (bind _getsave (`self.GetSave`))
  (bind _returnvalue (`GameplayStatics.CreateSaveGameObject` null))
  (bind _output_get (set `self.GetSave` _returnvalue))
  (set `/Game/Blueprints/GameInstances/LevelVariables_GI.Level1Clear` (`self.Level1Cleared`) _output_get)
  (set `/Game/Blueprints/GameInstances/LevelVariables_GI.Level2Clear` (`self.Level2Cleared`) _getsave)
  (set `/Game/Blueprints/GameInstances/LevelVariables_GI.Level3Clear` (`self.Level3Cleared`) _getsave)
  (`GameplayStatics.SaveGameToSlot` _getsave "VictorSlot"))